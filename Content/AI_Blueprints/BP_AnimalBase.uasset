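; Base animal character that supplies random patrol destinations along a BP_PatrolRoute spline and an event to set walk speed.
; On BeginPlay it picks a random route from the level if none is assigned and prints its name.
; GetPatrolPoint returns a random spline point's world location, offsetting on a LastSpot match, though LastSpot is never written here.
; An older back-and-forth index stepper remains in that function, disconnected.
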(event Custom|SetSpeed
  (params (Speed :type Float%20%28double-precision%29))
  (Variables|/Script/Engine.CharacterMovementComponent|SetMaxWalkSpeed (Variables|Character|GetCharacterMovement) Speed))

(event EventBeginPlay
  (Utilities|IsValid (Variables|Default|GetPatrol%20Route)
    (:Is%20Not%20Valid
      (bind _outactors (Actor|GetAllActorsOfClass "/Game/AI_Blueprints/BP_PatrolRoute.BP_PatrolRoute_C"))
      (bind _output_get (Variables|Default|SetPatrol%20Route (.OutItem (Utilities|Array|Random _outactors))))
      (Development|PrintString (Utilities|GetDisplayName _output_get) true true "(R=0.000000,G=0.660000,B=1.000000,A=1.000000)" 1e+01))))

(event Collision|EventActorBeginOverlap
  (params (OtherActor :type Actor%20Object%20Reference)))

(event EventTick
  (params (DeltaSeconds :type Float%20%28single-precision%29)))

(fn ConstructionScript)

(fn GetPatrolPoint
  (bind _patrol_route (Variables|Default|GetPatrol%20Route))
  (bind _spline (Variables|/Game/AI_Blueprints/BP_PatrolRoute.BP_PatrolRoute_C|GetSpline _patrol_route))
  (bind _returnvalue (Spline|GetNumberOfSplinePoints _spline))
  (bind _returnvalue_2 (Math|Random|RandomIntegerinRange 1 _returnvalue))
  (bind _output_get (Variables|Default|SetPatrolIndex _returnvalue_2))
  (if (== _returnvalue_2 (Variables|Default|GetLastSpot))
    (Variables|Default|SetPatrolIndex (+ _output_get (Math|Random|RandomIntegerinRange -2 2)))
    (if (> (+ _output_get (Math|Random|RandomIntegerinRange -2 2)) _returnvalue)
      (Variables|Default|SetPatrolIndex _returnvalue)))
  (return (Spline|GetLocationatSplinePoint (Variables|/Game/AI_Blueprints/BP_PatrolRoute.BP_PatrolRoute_C|GetSpline (Variables|Default|GetPatrol%20Route)) (Variables|Default|GetPatrolIndex) "World")))