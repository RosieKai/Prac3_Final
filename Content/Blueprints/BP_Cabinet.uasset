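; BP_Cabinet is a cabinet actor whose large and small left and right doors swing open and closed automatically from BeginPlay.
; OpenClose uses a FlipFlop to alternate a Timeline between Play and Reverse, with its track scaling opposite yaw rotations up to 90 degrees for each side.
; The Timeline's Finished pin calls OpenClose again, so the motion loops continuously without player input.
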(event Custom|OpenClose
  (Utilities|FlowControl|FlipFlop
    (:A
      (bind _newtrack_0 (Timeline|Timeline Play)
        (:Update
          (Transformation|SetRelativeRotation (Variables|Default|GetDoor_L) (Math|Rotator|MakeRotator 0.0 0.0 (* _newtrack_0 9e+01)) false false)
          (Transformation|SetRelativeRotation (Variables|Default|GetDoor_R) (Math|Rotator|MakeRotator 0.0 0.0 (* _newtrack_0 -9e+01)) false false))
        (:Finished
          (CallFunction|OpenClose))))
    (:B
      (Timeline|Timeline Reverse))))

(event EventBeginPlay
  (CallFunction|OpenClose))

(fn ConstructionScript)