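; BP_CineCam is a cinematic camera actor that, when its ActiveCam flag is set, becomes the player's view and spins continuously.
; On BeginPlay it switches the first player controller's view target to itself and starts SpinCam.
; A timeline drives the actor's yaw through 360 degrees and restarts itself on finish to loop the rotation.
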(event Custom|Spin%20Cam
  (bind _newtrack_1 (Timeline|Timeline PlayFromStart)
    (:Update
      (Transformation|SetActorRotation (Math|Rotator|MakeRotator 0.0 0.0 (* _newtrack_1 3.6e+02))))
    (:Finished
      (CallFunction|SpinCam))))

(event EventBeginPlay
  (if (Variables|Default|GetActiveCam)
    (Game|Player|SetViewTargetwithBlend (Game|GetPlayerController 0) self 0.0 "VTBlend_Linear" 0.0 false)
    (CallFunction|SpinCam)))

(fn ConstructionScript)