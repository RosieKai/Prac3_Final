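; Door actor that starts swinging when play begins and keeps opening and closing in a loop.
; An IsToybox flag selects between a -90 degree roll hinge for toybox lids and a 90 degree yaw swing for regular doors.
; Each branch uses a FlipFlop to alternate playing and reversing its own timeline, whose Finished output calls OpenClose again to sustain the cycle.
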(event Custom|OpenClose
  (if (Variables|Default|GetIsToybox)
    (Utilities|FlowControl|FlipFlop
      (:A
        (bind _newtrack_0 (Timeline|Timeline_0 Play)
          (:Update
            (Transformation|SetRelativeRotation (Variables|Default|GetDoor) (Math|Rotator|MakeRotator (* _newtrack_0 -9e+01) 0.0 0.0) false false))
          (:Finished
            (CallFunction|OpenClose))))
      (:B
        (Timeline|Timeline_0 Reverse)))
    (else
      (Utilities|FlowControl|FlipFlop
        (:A
          (bind _newtrack_0_2 (Timeline|Timeline Play)
            (:Update
              (Transformation|SetRelativeRotation (Variables|Default|GetDoor) (Math|Rotator|MakeRotator 0.0 0.0 (* _newtrack_0_2 9e+01)) false false))
            (:Finished
              (CallFunction|OpenClose))))
        (:B
          (Timeline|Timeline Reverse))))))

(event EventBeginPlay
  (CallFunction|OpenClose))

(fn ConstructionScript)