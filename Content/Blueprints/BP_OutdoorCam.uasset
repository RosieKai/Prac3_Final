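; BP_OutdoorCam is an actor with a cine camera that spins through yaw rotation, apparently for an outdoor view.
; After a short delay on BeginPlay, it casts the player to BP_ThirdPersonCharacter, activates both that character's follow camera and its own CineCamera, then starts the spin.
; A timeline drives the actor's yaw, mapping its track value to degrees of a full turn.
; It also prints a debug string.
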(event Custom|Spin%20Cam
  (bind _newtrack_1 (Timeline|Timeline PlayFromStart)
    (:Update
      (Transformation|SetActorRotation (Math|Rotator|MakeRotator 0.0 0.0 (* _newtrack_1 3.6e+02))))))

(event EventBeginPlay
  (Utilities|FlowControl|Delay 0.2)
  (bind _asbp_third_person_character (Utilities|Casting|CastToBP_ThirdPersonCharacter (Game|GetPlayerCharacter 0)))
  (Components|Activation|SetActive (Variables|/Game/ThirdPerson/Blueprints/BP_ThirdPersonCharacter.BP_ThirdPersonCharacter_C|GetFollowCamera _asbp_third_person_character) true false)
  (Components|Activation|SetActive (Variables|Default|GetCineCamera) true false)
  (CallFunction|SpinCam)
  (Development|PrintString "Hello"))

(fn ConstructionScript)